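; BP_Marine is a player pawn with world-axis movement input and intended twin-stick aiming.
; Each Tick, UpdatePlayerAim would set player 0's control yaw from the right and up thumbstick axes via Atan2, gated by a deadzone check.
; That check's length comparison is disconnected from its entry, so as wired it returns the default false and aim never updates.
; GetMouseVelocity is an unfinished stub.
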(event `InputAxis|MoveForward`
  (params (AxisValue :type "Float (single-precision)"))
  (`self.AddMovementInput` (1.0 0.0 0.0) AxisValue))

(event `InputAxis|MoveRight`
  (params (AxisValue :type "Float (single-precision)"))
  (`self.AddMovementInput` (0.0 -1.0 0.0) AxisValue))

(event `self.ReceiveTick`
  (params (DeltaSeconds :type "Float (single-precision)"))
  (`self.Update Player Aim`))

(fn `Get Mouse Velocity`)

(fn `Is Thumbstick Above Deadzone`
  (returns (ReturnValue :type Boolean)))

(fn `Update Player Aim`
  (locals (NewLocalVar_0 :type "Float (double-precision)" :default 0.0))
  (if (`self.Is Thumbstick Above Deadzone`)
    (`Controller.SetControlRotation` (`GameplayStatics.GetPlayerController` 0) (`KismetMathLibrary.MakeRotator` 0.0 0.0 (`KismetMathLibrary.DegAtan2` (`self.GetInputAxisValue`) (`self.GetInputAxisValue`))))))

(fn `UserConstructionScript`)